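; BP_Crystal is a damageable map crystal that bobs in place and shrinks as it loses health.
; On BeginPlay it fills health, plays a crystal sound and starts a timeline, restarted on finish, that moves the mesh and billboard vertically.
; AnyDamage lowers clamped health and plays a Wilhelm sound.
; Tick sets mesh scale to the health ratio each frame and destroys the actor at zero health.
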(event `self.ReceiveBeginPlay`
  (set `self.Health` (`self.HealthMax`))
  (`GameplayStatics.PlaySoundAtLocation` "/Game/Sounds/Sound_Cues/Crystal_Sound.Crystal_Sound" (`SceneComponent.K2_GetComponentLocation` (`self.SM_Crytal`)) (struct) 1.0 1.0 0.0 null null null null)
  (bind (_direction _ypossphere) (`Timeline|Timeline_0` :!label _label)
    (:`Update`
      (`SceneComponent.K2_SetRelativeLocation` (`self.SM_2xBillboard_v1`) (`KismetMathLibrary.MakeVector` 0.0 0.0 (* _ypossphere 7.0)) false false)
      (`SceneComponent.K2_SetRelativeLocation` (`self.SM_Crytal`) (`KismetMathLibrary.MakeVector` 0.0 0.0 (* _ypossphere 7.0)) false false))
    (:`Finished`
      (goto _label :!via `PlayFromStart`))))

(event `self.ReceiveTick`
  (params (DeltaSeconds :type "Float (single-precision)"))
  (`SceneComponent.SetWorldScale3D` (`self.SM_Crytal`) (`KismetMathLibrary.Conv_DoubleToVector` (/ (`self.Health`) (`self.HealthMax`))))
  (if (<= (`self.Health`) 0.0)
    (`self.K2_DestroyActor`)))

(event `self.ReceiveAnyDamage`
  (params (Damage :type "Float (single-precision)") (DamageType :type "DamageType Object Reference") (InstigatedBy :type "Controller Object Reference") (DamageCauser :type "Actor Object Reference"))
  (set `self.Health` (`KismetMathLibrary.FClamp` (- (`self.Health`) Damage) 0.0 (`self.HealthMax`)))
  (`GameplayStatics.PlaySoundAtLocation` "/Game/Sounds/Wilhelm_Sound.Wilhelm_Sound" (`SceneComponent.K2_GetComponentLocation` (`self.SM_Crytal`)) (struct) 1.0 1.0 0.0 null null null null))

(fn `UserConstructionScript`)