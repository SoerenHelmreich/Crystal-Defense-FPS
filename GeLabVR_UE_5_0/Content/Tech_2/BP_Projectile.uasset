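; BP_Projectile is a grenade-like projectile that deals area damage when it overlaps an actor tagged Enemy or Landscape.
; Launch propels its Sphere forward with an impulse.
; On overlap it asks VRGameState to spawn an AOE, whose hit callback sends DamageMessage to each hit actor.
; It also plays smoke and sound, then destroys itself after a short delay; an older ApplyDamage explosion path is left disconnected.
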(event `self.ReceiveActorBeginOverlap`
  (params (OtherActor :type "Actor Object Reference"))
  (bind _returnvalue (`SceneComponent.K2_GetComponentLocation` (`self.Sphere`)))
  (if (or (`self.ActorHasTag` OtherActor "Enemy") (`self.ActorHasTag` OtherActor "Landscape"))
    (bind _asvrgame_state (cast `/Game/Tech/VRGameState` (`GameplayStatics.GetGameState`)))
    (`/Game/Tech/VRGameState.Spawn AOE` _asvrgame_state _returnvalue 400.0 false (`GameplayStatics.GetPlayerPawn` 0) (delegate `CustomEvent_0`) 0.0 (struct :`R` 0.925347 :`G` 0.136553 :`B` 0.26943 :`A` 1.0))
    (bind _returnvalue_2 (`NiagaraFunctionLibrary.SpawnSystemAtLocation` "/Game/Particles/NS_SmokeBurst.NS_SmokeBurst" _returnvalue (struct) (2.0 2.0 2.0)))
    (`GameplayStatics.PlaySoundAtLocation` "/Game/Sounds/Granate_Sound.Granate_Sound" _returnvalue (struct) 1.0 1.0 0.0 null null null null)
    (`KismetSystemLibrary.Delay` 1.4)
    (`ActorComponent.K2_DestroyComponent` _returnvalue_2)
    (`self.K2_DestroyActor`)))

(event `CustomEvent_0`
  (params (`Hit Actor` :type "Actor Object Reference"))
  (message `/Game/Tech/BP_HealthInterface.Damage` `Hit Actor` 50.0))

(fn `Launch`
  (bind _sphere (`self.Sphere`))
  (`PrimitiveComponent.AddImpulse` _sphere (* (`SceneComponent.GetForwardVector` _sphere) (3000.0 3000.0 3000.0)) "None" false))

(fn `UserConstructionScript`)